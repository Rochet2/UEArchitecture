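; Battery pickup Blueprint that adds its BatteryPower to the player character through UpdatePower when overlapped.
; A valid MyProject5Character overlap while active deactivates the pickup, so it only fires once.
; A sequence then starts a timeline that scales the mesh and destroys the actor when finished, spawns an attached particle emitter and launches the mesh upward with a velocity-change impulse.
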(event Collision|EventActorBeginOverlap
  (params (OtherActor :type Actor%20Object%20Reference))
  (Utilities|IsValid OtherActor
    (:Is%20Valid
      (bind _asmy_project_5character (Utilities|Casting|CastToMyProject5Character OtherActor))
      (if (Class|Pickup|IsActive self)
        (Class|Pickup|SetActive false)
        (Utilities|FlowControl|Sequence
          (:then_0
            ;[1 1 1] Scale down and delete
            (bind _newtrack_1 (Timeline|Timeline_0 Play)
              (:Update
                (Transformation|SetWorldScale3D (Variables|Default|GetPickupMesh self) (Math|Conversions|ToVector(Float) _newtrack_1)))
              (:Finished
                (Actor|DestroyActor))))
          (:then_1
            ;[1 1 1] Spawn visual emitter
            (bind _returnvalue (Effects|SpawnEmitterAttached 0 (Variables|Default|GetScene2) "None" "0, 0, 0" "0, 0, 0" "2.000000,2.000000,2.000000"))
            (Utilities|FlowControl|Sequence
              (:then_0
                (Variables|/Script/Engine.SceneComponent|SetbAbsoluteScale _returnvalue false))
              (:then_1
                (Variables|/Script/Engine.SceneComponent|SetbAbsoluteRotation _returnvalue true))))
          (:then_2
            ;[1 1 1] Push object upwards
            (Physics|AddImpulse (Variables|Default|GetPickupMesh) "0, 0,500.000000" "None" true))
          (:then_3
            (Class|MyProject5Character|UpdatePower _asmy_project_5character (Variables|Default|GetBatteryPower self))))))))

(fn ConstructionScript)